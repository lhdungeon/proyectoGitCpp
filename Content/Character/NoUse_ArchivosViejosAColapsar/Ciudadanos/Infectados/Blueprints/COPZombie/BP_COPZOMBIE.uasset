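; Infected cop zombie enemy Blueprint that bites, takes damage and rewards kills, filed under an unused-assets folder.
; MordidaZOMBIE sphere-traces at the mouth socket and applies radial bite damage.
; AnyDamage and DañoInterface share damage handling: survivors briefly show a health widget, while death removes movement and sensing, then grants experience, kill count and rewards.
; Tick removes dead bodies once flagged as searched, with a timed fallback flag.
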(event Custom|MordidaZOMBIE
  (bind _mordida (Variables|Default|GetMordida))
  (bind _returnvalue (Transformation|GetSocketLocation _mordida "Mordida"))
  ;[1 1 1] Apply Damage
  (bind _outactors (Actor|GetAllActorsOfClass 0))
  (bind _returnvalue_2 (Collision|SphereTraceByChannel _returnvalue _returnvalue 75.0 "TraceTypeQuery2" false _outactors "None"))
  (if _returnvalue_2
    (Game|Damage|ApplyRadialDamage (Variables|Default|GetDañoBase) _returnvalue 75.0 0 _outactors 0 0 false "ECC_Camera")))

(event EventBeginPlay
  (|CallParentFunction)
  (Variables|Default|SetrefZombieInstanciaAnimacione (Components|SkeletalMesh|GetAnimInstance (Variables|Character|GetMesh))))

(event Game|Damage|EventAnyDamage
  (params (Damage :type Float%20%28single-precision%29) (DamageType :type Damage%20Type%20Object%20Reference) (InstigatedBy :type Controller%20Object%20Reference) (DamageCauser :type Actor%20Object%20Reference))
  ;[1 1 1] ANY DAMAGE
  (bind _vida0_ (CallFunction|DañoRecibidoFuncion Damage))
  (if _vida0_
    (bind _returnvalue (UserInterface|CreateWidget 0))
    (Variables|Default|SetSaludEnemigo _returnvalue (Variables|Default|GetSalud))
    (Variables|Default|SetSaludMAXEnemigo _returnvalue (Variables|Default|GetSaludMAX))
    (Components|DestroyComponent (Variables|Character|GetCharacterMovement))
    ;;[1 1 1] Añadir Funcion Para revisar cuerpos abatidos y luego setear esta variable -------------------------------------->     ↓
    (Variables|Default|SetRecibioDaño? false)
    (Utilities|MuerteExpConteo)
    (Utilities|FlowControl|Delay 0.5)
    (CallFunction|PremiosFuncion)
    (Variables|Default|SetCuerpoRevisado? true)
    (else
      (Variables|Default|SetRecibioDaño? true)
      (bind _returnvalue_2 (UserInterface|CreateWidget 0))
      (Variables|Default|SetSaludEnemigo _returnvalue_2 (Variables|Default|GetSalud))
      (Variables|Default|SetSaludMAXEnemigo _returnvalue_2 (Variables|Default|GetSaludMAX))
      (UserInterface|Viewport|AddtoPlayerScreen _returnvalue_2)
      (Utilities|FlowControl|Delay 0.3)
      (Variables|Default|SetRecibioDaño? false)
      (Widget|RemovefromParent _returnvalue_2))))

(event EventRevisarCuerpo
  ;[1 1 1] ANY DAMAGE
  (|CallParentFunction))

(event EventTick
  (params (DeltaSeconds :type Float%20%28single-precision%29))
  ;[1 1 1] TICK + DESAPARICION
  (Utilities|FlowControl|Sequence
    (:then_0
      (if (Variables|Default|GetMuerto?)
        (if (Variables|Default|GetCuerpoRevisado?)
          (Utilities|FlowControl|Delay 0.2)
          (CallFunction|FuncionDesaparecerAlmorir)
          (else
            (Utilities|FlowControl|Delay 6e+01)
            (Variables|Default|SetCuerpoRevisado? true)))))))

(event EventDañoInterface
  (params (Daño :type Float%20%28single-precision%29) (instigador :type Actor%20Object%20Reference))
  ;[1 1 1] ANY DAMAGE
  (if (not (or (Variables|Default|GetRecibioDaño?) (Variables|Default|GetMuerto?)))
    (bind _vida0_ (CallFunction|DañoRecibidoFuncion Daño))
    (if _vida0_
      (bind _returnvalue (UserInterface|CreateWidget 0))
      (Variables|Default|SetSaludEnemigo _returnvalue (Variables|Default|GetSalud))
      (Variables|Default|SetSaludMAXEnemigo _returnvalue (Variables|Default|GetSaludMAX))
      (Components|DestroyComponent (Variables|Character|GetCharacterMovement))
      ;;[1 1 1] Añadir Funcion Para revisar cuerpos abatidos y luego setear esta variable -------------------------------------->     ↓
      (Variables|Default|SetRecibioDaño? false)
      (Utilities|MuerteExpConteo)
      (Utilities|FlowControl|Delay 0.5)
      (CallFunction|PremiosFuncion)
      (Variables|Default|SetCuerpoRevisado? true)
      (else
        (Variables|Default|SetRecibioDaño? true)
        (bind _returnvalue_2 (UserInterface|CreateWidget 0))
        (Variables|Default|SetSaludEnemigo _returnvalue_2 (Variables|Default|GetSalud))
        (Variables|Default|SetSaludMAXEnemigo _returnvalue_2 (Variables|Default|GetSaludMAX))
        (UserInterface|Viewport|AddtoPlayerScreen _returnvalue_2)
        (Utilities|FlowControl|Delay 0.3)
        (Variables|Default|SetRecibioDaño? false)
        (Widget|RemovefromParent _returnvalue_2)))))

(fn ConstructionScript
  (Transformation|AttachComponentToComponent (Variables|Default|GetManoder) (Variables|Character|GetMesh) "RightHand" "KeepRelative" "KeepRelative" "KeepRelative" true)
  (Transformation|AttachComponentToComponent (Variables|Default|GetManoizq) (Variables|Character|GetMesh) "LeftHand" "KeepRelative" "KeepRelative" "KeepRelative" true)
  (Transformation|AttachComponentToComponent (Variables|Default|GetMordida) (Variables|Character|GetMesh) "Mordida" "KeepRelative" "KeepRelative" "KeepRelative" true))