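; Male player character Blueprint that adds weapon setup and damage response to a parent handling hunger, thirst, fatigue, items and equipping.
; BeginPlay caches the anim instance and spawns a hidden weapon actor.
; AnyDamage asks the GameInstance for death: fatal hits clear widgets, then show another and pause the game after a delay; others play a montage and widget.
; Head-turning toward nearby actors is unfinished and disconnected, with empty overlap events.
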(event OnComponentBeginOverlap(Sphere)
  (params (OverlappedComponent :type Primitive%20Component%20Object%20Reference) (OtherActor :type Actor%20Object%20Reference) (OtherComp :type Primitive%20Component%20Object%20Reference) (OtherBodyIndex :type Integer) (bFromSweep :type Boolean) (SweepResult :type Hit%20Result%20Structure%20%28by%20ref%29))
  ;[0 0.9737 1] """""TERMINARRRR """""FuncionParaRotar Cabeza Del Jugador Hacia los Demas actores
)

(event OnComponentEndOverlap(Sphere)
  (params (OverlappedComponent :type Primitive%20Component%20Object%20Reference) (OtherActor :type Actor%20Object%20Reference) (OtherComp :type Primitive%20Component%20Object%20Reference) (OtherBodyIndex :type Integer))
  ;[0 0.9737 1] """""TERMINARRRR """""FuncionParaRotar Cabeza Del Jugador Hacia los Demas actores
)

(event Custom|TomarItems
  ;[0.126 1 0] Custom events HEREDADOS
  (|CallParentFunction))

(event Game|Damage|EventAnyDamage
  (params (Damage :type Float%20%28single-precision%29) (DamageType :type Damage%20Type%20Object%20Reference) (InstigatedBy :type Controller%20Object%20Reference) (DamageCauser :type Actor%20Object%20Reference))
  ;[0 0.2242 1] Any Damage O Blueprint Interfaces?¿?¿
  (bind _vida0_ (CallFunction|Daño (Variables|Default|GetrefGAMEINSTANCE) Damage))
  (if _vida0_
    (Variables|Default|SetMuerto? true)
    (Class|KismetSystemLibrary|PauseTimer (Variables|Default|GetArmaEquipada) "GuiaDeAtaque")
    (Viewport|RemoveAllWidgets)
    (Utilities|FlowControl|Delay 2.9)
    (bind _returnvalue (UserInterface|CreateWidget 0))
    (UserInterface|Viewport|AddtoViewport _returnvalue 0)
    (Game|SetGamePaused true)
    (else
      (Variables|Default|SetMuerto? false)
      (Animation|PlayAnimMontage 0 1.0 "None")
      (bind _returnvalue_2 (UserInterface|CreateWidget 0))
      (UserInterface|Viewport|AddtoViewport _returnvalue_2 0)
      (Class|KismetSystemLibrary|PauseTimer (Variables|Default|GetArmaEquipada) "GuiaDeAtaque"))))

(event EventBeginPlay
  ;[1 0 0.4851] BeginPlay
  (|CallParentFunction)
  (Variables|Default|SetRefAnimInstanceMale (Components|SkeletalMesh|GetAnimInstance (Variables|Character|GetMesh)))
  (bind _returnvalue (Game|SpawnActorfromClass 0 (Variables|Default|GetTransform%20Arma) "Undefined" 0 0))
  (bind _output_get (Variables|Default|SetActorArmaRef _returnvalue))
  (Rendering|SetActorHiddenInGame _output_get true)
  (Variables|Default|SetEquipaMelee? false))

(event EventSed
  ;[0.126 1 0] Custom events HEREDADOS
  (|CallParentFunction))

(event EventSedOHambre?
  ;[0.126 1 0] Custom events HEREDADOS
  (|CallParentFunction))

(event EventTick
  (params (DeltaSeconds :type Float%20%28single-precision%29))
  ;[1 0 0.4851] EventTick
  (|CallParentFunction 0.0))

(event EventDecrementarCansancio
  ;[0.126 1 0] Custom events HEREDADOS
  (|CallParentFunction))

(event EventRegenerarCansancio
  ;[0.126 1 0] Custom events HEREDADOS
  (|CallParentFunction))

(event EventEquiparDesequipar
  ;[0.126 1 0] Custom events HEREDADOS
  (|CallParentFunction))

(event EventHambre
  ;[0.126 1 0] Custom events HEREDADOS
  (|CallParentFunction))

(fn ConstructionScript)

(fn FuncionHambre
  (params (RanFloatMin :type Float%20%28single-precision%29) (RanFloatMAX :type Float%20%28single-precision%29))
  (bind _sedientohambriento_ (|CallParentFunction RanFloatMin RanFloatMAX))
  (return _sedientohambriento_))

(fn VerificarArmas
  (|CallParentFunction))

(fn FuncionSed
  (params (RanMin :type Float%20%28single-precision%29) (RanMax :type Float%20%28single-precision%29))
  (bind _sedientohambriento_ (|CallParentFunction RanMin RanMax))
  (return _sedientohambriento_))

(fn RotacionHead
  (bind _returnvalue (Pawn|GetControlRotation :!class /Script/Engine.Pawn))
  (bind _returnvalue_2 (Transformation|GetActorRotation))
  (bind _returnvalue_3 (- (.yaw _returnvalue) (.yaw _returnvalue_2)))
  (bind _returnvalue_4 (Math|Float|ClampAngle _returnvalue_3 -179.899994 -1.8e+02))
  (bind _asbp_anim_male (Utilities|Casting|CastTo (Variables|Default|GetRefAnimInstanceMale)))
  (Variables|Default|SetRotacionCabeza _asbp_anim_male (Math|Rotator|MakeRotator (- 0.0 (.pitch _returnvalue)) 0.0 _returnvalue_4))
  (if (not (> _returnvalue_4 9e+01))
    (if (< _returnvalue_4 -9e+01)
      _)))