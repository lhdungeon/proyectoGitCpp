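; Base Blueprint for infected enemies, apparently retired, with empty casts and disconnected initialization.
; PawnSensing feeds AIMoveTo, which raises a timed attack flag on arrival and retries on failure.
; Functions provide defense-reduced damage, corpse sinking, one-time random loot from a searched body, and a GameInstance enemy count that spawns emitters when the wave clears.
; SeteoDeValores would scale stats and speed by random level, but its EventGraph call never runs.
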(event OnSeePawn(PawnSensing)
  (params (Pawn :type Pawn%20Object%20Reference))
  (InfectedParent|PawnSensingFuncion Pawn))

(event Custom|BuscarPersonaje
  (params (Pawn :type Pawn%20Object%20Reference))
  ;[1 1 1] BuscaPersonaje
  (if (not (Variables|InfectedParent|GetMuerto?))
    (AI|AIMoveTo self "0, 0, 0" Pawn 4e+01 false
      (:OnSuccess
        (Variables|InfectedParent|Setatacando? true)
        (Utilities|FlowControl|Delay 2.27)
        (Variables|InfectedParent|Setatacando? false))
      (:OnFail
        (CallFunction|BuscarPersonaje Pawn)
        (Variables|InfectedParent|Setatacando? false)))))

(event Custom|DañoInterface_1)

(event EventBeginPlay
  ;[1 1 1] BeginPlay
)

(fn ConstructionScript)

(fn DañoRecibidoFuncion
  (params (DañoRecibido :type Float%20%28single-precision%29))
  (bind _output_get (Variables|InfectedParent|SetDañoRecibido (- DañoRecibido (Math|Conversions|ToFloat(Integer) (Variables|InfectedParent|GetDefensaEnemigo)))))
  (bind _output_get_2 (Variables|InfectedParent|SetSalud (Math|Float|Clamp(Float) (- (Variables|InfectedParent|GetSalud) _output_get) 0.0 (Variables|InfectedParent|GetSaludMAX))))
  (return (<= _output_get_2 0.0) _output_get))

(fn Muerto
  (Variables|InfectedParent|SetMuerto? true)
  (return))

(fn ExperienciaPostMortem)

(fn FuncionDesaparecerAlmorir
  (bind _returnvalue (Transformation|GetActorLocation))
  (bind _returnvalue_2 (- (.z _returnvalue) 0.25))
  (bind _returnvalue_3 (<= _returnvalue_2 2.2e+02))
  (if (Variables|InfectedParent|GetMuerto?)
    (Collision|SetCollisionEnabled (Variables|Collision|GetCapsuleComponent) "PhysicsOnly")
    (Transformation|SetActorLocation (Math|Vector|MakeVector (.x _returnvalue) (.y _returnvalue) _returnvalue_2) false false)
    (if _returnvalue_3
      (Actor|DestroyActor)
      (return _returnvalue_3))))

(fn PawnSensingFuncion
  (params (PawnMasc :type Pawn%20Object%20Reference))
  (bind _asbp_masculino (Utilities|Casting|CastTo PawnMasc))
  (CallFunction|BuscarPersonaje _asbp_masculino))

(fn ConteoDeEnemigos
  (bind _self self)
  (bind _returnvalue (Transformation|GetActorLocation _self))
  (bind _asgameinstance (Utilities|Casting|CastTo (Game|GetGameInstance)))
  (bind _output_get (Variables|Default|SetCantidadDeEnemigosEnPantalla _asgameinstance (- (Variables|Default|GetCantidadDeEnemigosEnPantalla _asgameinstance) 1)))
  (if (and (== (Variables|Default|GetCantidadDeEnemigosSPAWNED _asgameinstance) (Variables|Default|GetEnemigosAsPawned _asgameinstance)) (== _output_get 0))
    (Effects|SpawnEmitteratLocation 0 _returnvalue "0, 0, 0" "5.000000,5.000000,5.000000")
    (Effects|SpawnEmitteratLocation 0 _returnvalue "0, 0, 0" "100.000000,100.000000,100.000000")))

(fn PremiosFuncion
  (bind _mesh (Variables|Character|GetMesh))
  (bind _returnvalue (Transformation|GetWorldLocation _mesh))
  (if (Variables|InfectedParent|GetMuerto?)
    (Game|SpawnActorfromClass (Utilities|Array|Get(acopy) (Variables|InfectedParent|GetPremiosVar) (Math|Random|RandomIntegerinRange 0 (Variables|InfectedParent|GetRandomDePremios))) (Math|Transform|MakeTransform (Math|Vector|MakeVector (.x _returnvalue) (.y _returnvalue) (+ (.z _returnvalue) 5e+01)) "0, 0, 0" "1,1,1") "Undefined" 0 0)))

(fn RevisarCuerpo
  (if (Variables|InfectedParent|GetMuerto?)
    (if (not (Variables|InfectedParent|GetCuerpoRevisado?))
      (InfectedParent|PremiosFuncion)
      (Variables|InfectedParent|SetCuerpoRevisado? true)
      (return))))