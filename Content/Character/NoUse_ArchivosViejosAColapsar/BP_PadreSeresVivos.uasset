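; Parent character Blueprint for living beings, filed among unused old files, handling health, damage and an info widget.
; BeginPlay fills health to maximum; a sphere overlap toggles the info widget component and creates or removes a health widget.
; Daño subtracts defense from damage, clamps health, plays a health-loss animation on a newly created widget and returns whether health is depleted.
; AnyDamage is empty, and the death/montage branch is disconnected.
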(event OnComponentBeginOverlap(Sphere)
  (params (OverlappedComponent :type Primitive%20Component%20Object%20Reference) (OtherActor :type Actor%20Object%20Reference) (OtherComp :type Primitive%20Component%20Object%20Reference) (OtherBodyIndex :type Integer) (bFromSweep :type Boolean) (SweepResult :type Hit%20Result%20Structure%20%28by%20ref%29))
  (Utilities|Casting|CastTo OtherActor)
  (Rendering|SetVisibility (Variables|Default|GetWdInfo) true false)
  (bind _returnvalue (UserInterface|CreateWidget 0))
  (bind _output_get (Variables|SeresVivientes|SetSalud _returnvalue (Variables|SeresVivientes|GetSalud)))
  (Development|PrintString (Utilities|String|ToString(Float) _output_get)))

(event OnComponentEndOverlap(Sphere)
  (params (OverlappedComponent :type Primitive%20Component%20Object%20Reference) (OtherActor :type Actor%20Object%20Reference) (OtherComp :type Primitive%20Component%20Object%20Reference) (OtherBodyIndex :type Integer))
  (Utilities|Casting|CastTo OtherActor)
  (Rendering|SetVisibility (Variables|Default|GetWdInfo) false false)
  (Widget|RemovefromParent (stale OnComponentBeginOverlap(Sphere) _returnvalue)))

(event EventBeginPlay
  ;[1 1 1] Event BEGINPLAY
  (Variables|SeresVivientes|SetSalud (Variables|SeresVivientes|GetSaludMax))
  (bind _asgameinstance (Utilities|Casting|CastTo (Game|GetGameInstance)))
  (Variables|SeresVivientes|SetrefGAMEINSTANCE 0 _asgameinstance)
  (UserInterface|CreateWidget 0))

(event EventTick
  (params (DeltaSeconds :type Float%20%28single-precision%29)))

(event Game|Damage|EventAnyDamage
  (params (Damage :type Float%20%28single-precision%29) (DamageType :type Damage%20Type%20Object%20Reference) (InstigatedBy :type Controller%20Object%20Reference) (DamageCauser :type Actor%20Object%20Reference))
  ;[1 1 1] Event ANY DAMAGE
)

(fn ConstructionScript)

(fn Daño
  (params (DañoRecibido :type Float%20%28single-precision%29))
  (bind _output_get (Variables|SeresVivientes|SetDañorecibido (- DañoRecibido (Math|Conversions|ToFloat(Integer) (Variables|SeresVivientes|GetDefensaSeVi)))))
  (bind _output_get_2 (Variables|SeresVivientes|SetSalud (Math|Float|Clamp(Float) (- (Variables|SeresVivientes|GetSalud) _output_get) 0.0 (Variables|SeresVivientes|GetSaludMax))))
  (bind _returnvalue (UserInterface|CreateWidget 0))
  (UserInterface|Animation|PlayAnimation _returnvalue (Variables|Default|GetPerdidadesalud _returnvalue) 0.0 1 "Forward" 1.0 false)
  (return (<= _output_get_2 0.0)))